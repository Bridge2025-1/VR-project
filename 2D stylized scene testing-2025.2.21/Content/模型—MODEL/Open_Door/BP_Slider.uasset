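; BP_Slider is a VR grabbable slider that drives a target, likely a door given its Open_Door folder.
; Grabbing stores the motion controller and starts a 0.01-second looping timer, which is cleared on drop.
; Each tick shifts the box along local Y by the controller's relative offset, clamped between the first two spline points.
; It then sends the scaled Y position to the target through OpenMessage.
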(event OnGrabbed(GrabComponent)
  (params (Motion%20Controller :type Motion%20Controller%20Component%20Object%20Reference))
  (Variables|Default|SetMotion%20Controller Motion%20Controller)
  (bind _returnvalue (Utilities|Time|SetTimerbyFunctionName 0 "Replicate Position" 0.01 true))
  (Variables|Default|SetTimer _returnvalue))

(event OnDropped(GrabComponent)
  (Utilities|Time|ClearandInvalidateTimerbyHandle (Variables|Default|GetTimer))
  (Variables|Default|SetMotion%20Controller 0))

(fn ConstructionScript)

(fn ReplicatePosition
  (bind _spline (Variables|Default|GetSpline))
  (bind _box (Variables|Default|GetBox))
  (bind _relativelocation (Variables|/Script/Engine.SceneComponent|GetRelativeLocation _box))
  (Transformation|SetRelativeLocation _box (Math|Vector|MakeVector 0.0 (Math|Float|Clamp(Float) (+ (.y _relativelocation) (.y (.location (Math|Transform|MakeRelativeTransform (Math|Conversions|ToTransform(Vector) (Transformation|GetWorldLocation (Variables|Default|GetMotion%20Controller))) (Math|Conversions|ToTransform(Vector) (Transformation|GetWorldLocation (Variables|Default|GetBox))))))) (.y (Spline|GetLocationatSplinePoint _spline 0 "Local")) (.y (Spline|GetLocationatSplinePoint _spline 1 "Local"))) (.z _relativelocation)) false false)
  (Class|BPIAction|Open(Message) (Variables|Default|GetTarget) (* (.y (Variables|/Script/Engine.SceneComponent|GetRelativeLocation (Variables|Default|GetBox))) 2.3)))