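; VR bow actor whose string is drawn with a motion controller and fires an arrow on release.
; Grabbing GrabSpring starts a looping timer that slides ColliderString along local Y to follow the controller, clamped between two spline points, and normalizes that position into PullBack.
; Dropping stops the timer, resets the string, spawns Projectile1_Arrow at ArrowSpawnPoint and passes PullBack to ArrowSpeed.
; The Arrow component is hidden on both grab and drop.
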(event OnGrabbed(GrabSpring)
  (params (Motion%20Controller :type Motion%20Controller%20Component%20Object%20Reference))
  (Variables|Default|SetMotion%20Controller Motion%20Controller)
  (Rendering|SetVisibility (Variables|Default|GetArrow) false false)
  (bind _returnvalue (Utilities|Time|SetTimerbyFunctionName 0 "RelativePosistion" 0.02 true))
  (Variables|Default|SetTimer _returnvalue))

(event OnDropped(GrabSpring)
  (bind _arrowspawnpoint (Variables|Default|GetArrowSpawnPoint))
  (Utilities|FlowControl|Sequence
    (:then_0
      (Utilities|Time|ClearandInvalidateTimerbyHandle (Variables|Default|GetTimer))
      (Variables|Default|SetMotion%20Controller 0)
      (Transformation|SetRelativeLocation (Variables|Default|GetColliderString) (Math|Vector|MakeVector 0.0 1.7e+02 0.0) false false)
      (Rendering|SetVisibility (Variables|Default|GetArrow) false false))
    (:then_1
      (bind _returnvalue (Game|SpawnActorfromClass "/Game/模型—MODEL/Archer/Projectile1_Arrow.Projectile1_Arrow_C" (Math|Transform|MakeTransform (Transformation|GetWorldLocation _arrowspawnpoint) (Transformation|GetWorldRotation _arrowspawnpoint)) "Undefined" "MultiplyWithRoot" self (Game|Player|GetPlayerPawn 0)))
      (Default|ArrowSpeed _returnvalue (Variables|Default|GetPullBack)))
    (:then_2
      (Variables|Default|SetPullBack 0.0))))

(fn ConstructionScript)

(fn RelativePosistion
  (bind _colliderstring (Variables|Default|GetColliderString))
  (bind _spline (Variables|Default|GetSpline))
  (bind _colliderstring_2 (Variables|Default|GetColliderString))
  (bind _motion_controller (Variables|Default|GetMotion%20Controller))
  (bind _returnvalue (Transformation|GetWorldLocation _motion_controller))
  (bind _returnvalue_2 (Transformation|GetWorldLocation _colliderstring))
  (bind _returnvalue_3 (Spline|GetLocationatSplinePoint _spline 1 "Local"))
  (bind _returnvalue_4 (Spline|GetLocationatSplinePoint _spline 0 "Local"))
  (bind _relativelocation (Variables|/Script/Engine.SceneComponent|GetRelativeLocation _colliderstring_2))
  (bind _returnvalue_5 (Math|Conversions|ToTransform(Vector) _returnvalue))
  (bind _returnvalue_6 (Math|Conversions|ToTransform(Vector) _returnvalue_2))
  (bind _returnvalue_7 (Math|Transform|MakeRelativeTransform _returnvalue_5 _returnvalue_6))
  (bind _returnvalue_8 (+ (.y (.location _returnvalue_7)) (.y _relativelocation)))
  (bind _returnvalue_9 (Math|Float|Clamp(Float) _returnvalue_8 (.y _returnvalue_4) (.y _returnvalue_3)))
  (Transformation|SetRelativeLocation (Variables|Default|GetColliderString) (Math|Vector|MakeVector 0.0 _returnvalue_9 0.0) false false)
  (Variables|Default|SetPullBack (Math|Float|NormalizetoRange _returnvalue_9 (.y _returnvalue_4) (.y _returnvalue_3))))